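; BP_Plataform is a moving platform that travels between two points using an InterpToMovement component.
; The construction script offsets PointA and PointB along world X by per-point values, then adds their relative locations as control points.
; The Speed variable sets the movement's Duration, so larger values mean slower travel.
; The event graph holds no active logic, leaving runtime motion to the component.
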(fn `SetPointPosition`
  (params (Point :type "SceneComponent Object Reference") (X :type "Float (double-precision)"))
  (bind (_x _y _z) (`KismetMathLibrary.BreakVector3f` (`SceneComponent.K2_GetComponentLocation` Point)))
  (`SceneComponent.K2_SetWorldLocation` Point (`KismetMathLibrary.MakeVector` (+ X _x) _y _z) false false))

(fn `UserConstructionScript`
  (set `InterpToMovementComponent.Duration` (`self.Speed`) (`self.InterpToMovement`))
  (`self.SetPointPosition` (`self.PointA`) (`self.APositionX`))
  (`self.SetPointPosition` (`self.PointB`) (`self.BPositionX`))
  (`InterpToMovementComponent.AddControlPointPosition` (`self.InterpToMovement`) (`SceneComponent.RelativeLocation` (`self.PointA`)) true)
  (`InterpToMovementComponent.AddControlPointPosition` (`self.InterpToMovement`) (`SceneComponent.RelativeLocation` (`self.PointB`)) true))